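; BP_GameMode is the game mode that tracks kill-based stage progress and broadcasts game-state changes through event dispatchers.
; GameStart announces the start and initial kill count, while MonsterKilled increments the count, broadcasts it and signals stage clear when it equals the target.
; PlayerDied broadcasts game over.
; LoadLevel streams in SubLevel02 without blocking and RestartGame reopens the main level, both via object references.
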(event `GameStart`
  ; 게임 시작 이벤트
  (`self.OnGameStart`)
  (`self.OnKillCountUpdated` (`self.CurrentKills`) (`self.TargetKills`)))

(event `MonsterKilled`
  ; 몬스터가 죽었을 떄
  (bind _result (`/Engine/EditorBlueprintResources/StandardMacros.IncrementInt` (`self.CurrentKills`))
    (:`  `
      (`self.OnKillCountUpdated` _result (`self.TargetKills`))
      ; 스테이지 클리어 조건 확인 및 이벤트 발생
      (if (== (`self.CurrentKills`) (`self.TargetKills`))
        (`self.OnStageClear`)))))

(event `LoadLevel`
  ; 서브 레벨 로드
  (`GameplayStatics.LoadStreamLevelBySoftObjectPtr` "/Game/Maps/Game/SubLevel02.SubLevel02" true))

(event `PlayerDied`
  ; 게임 오버
  (`self.OnGameOver`))

(event `RestartGame`
  ; 게임 시작
  (`GameplayStatics.OpenLevelBySoftObjectPtr` "/Game/Maps/Game/MainLevel.MainLevel"))

(fn `UserConstructionScript`)