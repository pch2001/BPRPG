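; Bear monster character that drives a Locomotion, Chase, Attack and Dead state machine, mirrored to the AI Blackboard and setting walk speed.
; PawnSensing starts a chase on seeing the player, which ends when the target leaves sight radius.
; Player weapon overlaps trigger explosion and material flash, while any damage feeds a fixed amount to BPHPController.
; Its death event disables capsule collision, then dissolves and destroys the bear; separate events toggle attack collision.
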(event `self.ReceiveActorBeginOverlap`
  (params (OtherActor :type "Actor Object Reference")))

(event `self.ReceiveTick`
  (params (DeltaSeconds :type "Float (single-precision)"))
  (switch `/Game/Blueprints/Monster/EBearState` (`self.State_BP`)
    (:`NewEnumerator0`
      (`self.OnLocomotion`))
    (:`NewEnumerator1`
      (`self.OnChase`))))

(event `self.CapsuleComponent.OnComponentBeginOverlap`
  (params (OverlappedComponent :type "PrimitiveComponent Object Reference") (OtherActor :type "Actor Object Reference") (OtherComp :type "PrimitiveComponent Object Reference") (OtherBodyIndex :type Integer) (bFromSweep :type Boolean) (SweepResult :type "HitResult Structure (by ref)"))
  ; 맞았을때 피격효과
  (if (`self.ActorHasTag` OtherActor "PlayerWeapon")
    (`GameplayStatics.SpawnEmitterAtLocation` "/Game/Particles/P_Explosion.P_Explosion" (`self.K2_GetActorLocation`) (struct) (2.0 2.0 2.0))
    (bind (_direction _hitvalue) (`Timeline|HitEffect` :!via `PlayFromStart`)
      (:`Update`
        (`MeshComponent.SetScalarParameterValueOnMaterials` (`self.Mesh`) "HitValue" _hitvalue)))))

(event `self.ReceiveBeginPlay`
  ; 죽음 이벤트에 바인딩
  (add `/Game/Blueprints/Components/BP_HPController.OnDeadEvent` (`self.BP_HPController`) (delegate `ReceiveOnDead`)))

(event `self.ReceiveAnyDamage`
  (params (Damage :type "Float (single-precision)") (DamageType :type "DamageType Object Reference") (InstigatedBy :type "Controller Object Reference") (DamageCauser :type "Actor Object Reference"))
  ; 대미지 처리
  (`/Game/Blueprints/Components/BP_HPController.ReceiveDamage` (`self.BP_HPController`) 10.0))

(event `ReceiveOnDead`
  (bind _mesh (`self.Mesh`))
  ; 죽음 이벤트에 바인딩
  (`self.UpdateState` "NewEnumerator3")
  (`PrimitiveComponent.SetCollisionEnabled` (`self.CapsuleComponent`) "NoCollision")
  (`KismetSystemLibrary.Delay` 2.0)
  (bind (_direction _dissolve _hitvalue) (`Timeline|DeathEffect`)
    (:`Update`
      (`MeshComponent.SetScalarParameterValueOnMaterials` _mesh "Dissolve" _dissolve)
      (`MeshComponent.SetScalarParameterValueOnMaterials` _mesh "HitValue" _hitvalue))
    (:`Finished`
      (`self.K2_DestroyActor`))))

(event `self.PawnSensing.OnSeePawn`
  (params (Pawn :type "Pawn Object Reference"))
  ; 시야 감시
  (if (`|EnumEquality` (`self.State_BP`) "NewEnumerator0")
    (if (`self.ActorHasTag` Pawn "Player")
      (`BlackboardComponent.SetValueAsObject` (`AIController.Blackboard` (`AIBlueprintHelperLibrary.GetAIController` self)) (`self.TargetPlayerKey`) Pawn)
      (`self.UpdateState` "NewEnumerator1"))))

(event `UpdateState`
  (params (newState :type "/Game/Blueprints/Monster/EBearState Enum" :default "NewEnumerator0"))
  (bind _charactermovement (`self.CharacterMovement`))
  ; 상태변경 벤트
  (if (`|EnumInequality` (`self.State_BP`) "NewEnumerator3")
    (bind _output_get (set `self.State_BP` newState))
    (`BlackboardComponent.SetValueAsEnum` (`AIController.Blackboard` (`AIBlueprintHelperLibrary.GetAIController` self)) (`self.StateKey`) _output_get)
    (switch `/Game/Blueprints/Monster/EBearState` (`self.State_BP`)
      (:`NewEnumerator0`
        (set `CharacterMovementComponent.MaxWalkSpeed` 200.0 _charactermovement))
      (:`NewEnumerator1`
        (set `CharacterMovementComponent.MaxWalkSpeed` 300.0 _charactermovement))
      (:`NewEnumerator2`
        (set `CharacterMovementComponent.MaxWalkSpeed` 0.0 _charactermovement :!label _label))
      (:`NewEnumerator3`
        (goto _label)))))

(event `OnAttackCheckStart`
  ; 공격 판정 시작/종료
  (`PrimitiveComponent.SetCollisionEnabled` (`self.AttackCollision`) "QueryOnly"))

(event `OnAttackCheckEnd`
  ; 공격 판정 시작/종료
  (`PrimitiveComponent.SetCollisionEnabled` (`self.AttackCollision`) "NoCollision"))

(fn `OnAttack`)

(fn `OnChase`
  (bind _asactor (cast `Actor` (`BlackboardComponent.GetValueAsObject` (`AIBlueprintHelperLibrary.GetBlackboard` (`AIBlueprintHelperLibrary.GetAIController` self)) (`self.TargetPlayerKey`))))
  (if (> (`KismetMathLibrary.Vector_Distance` (`self.K2_GetActorLocation` _asactor) (`self.K2_GetActorLocation`)) (`PawnSensingComponent.SightRadius` (`self.PawnSensing`)))
    (`self.UpdateState` "NewEnumerator0")))

(fn `OnDead`)

(fn `OnLocomotion`)

(fn `UserConstructionScript`)