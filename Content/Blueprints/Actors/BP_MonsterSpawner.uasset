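; Monster spawner actor that spawns monsters at random attached spawn-point actors once the game starts.
; On BeginPlay it collects its attached actors as spawn points, binds to BP_GameMode's game-start event and takes TargetKills as the spawn target.
; After a start delay, a re-armed one-second timer spawns MonsterClass until the spawn count reaches the target, halting if that many monsters already exist.
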(event `self.ReceiveTick`
  (params (DeltaSeconds :type "Float (single-precision)")))

(event `self.ReceiveBeginPlay`
  (bind _spawnpoints (`self.SpawnPoints`))
  (for _array_element (`self.GetAttachedActors` true)
    (`KismetArrayLibrary.Array_Add` _spawnpoints _array_element)
    (if (> (`KismetArrayLibrary.Array_Length` _spawnpoints) 0)
      (bind _asbp_game_mode (cast `/Game/Blueprints/Character/BP_GameMode` (`GameplayStatics.GetGameMode`)))
      (add `/Game/Blueprints/Character/BP_GameMode.OnGameStart` _asbp_game_mode (delegate `OnGameStart`))
      (set `self.TargetSpawnCount` (`/Game/Blueprints/Character/BP_GameMode.TargetKills` _asbp_game_mode)))))

(event `OnGameStart`
  (`KismetSystemLibrary.Delay` (`self.GameStartWaitTime`))
  (`self.StartSpawning`))

(event `StartSpawning`
  (`KismetSystemLibrary.K2_SetTimerDelegate` (delegate `SpawnMonster`) 1.0))

(event `SpawnMonster`
  (bind _outactors (`GameplayStatics.GetAllActorsOfClass` (`self.MonsterClass`)))
  (if (< (`KismetArrayLibrary.Array_Length` _outactors) (`self.TargetSpawnCount`))
    (bind _returnvalue (`|SpawnActorFromClass` (`self.MonsterClass`) (`self.GetTransform` (`KismetArrayLibrary.Array_Random` (`self.SpawnPoints`))) "AlwaysSpawn" "MultiplyWithRoot" null null))
    (`/Engine/EditorBlueprintResources/StandardMacros.IsValid` _returnvalue
      (:`Is Valid`
        (bind _result (`/Engine/EditorBlueprintResources/StandardMacros.IncrementInt` (`self.SpawnCount`))
          (:`  `
            (if (< _result (`self.TargetSpawnCount`))
              (`self.StartSpawning`)))))
      (:`Is Not Valid`
        (`self.StartSpawning`)))))

(fn `UserConstructionScript`)