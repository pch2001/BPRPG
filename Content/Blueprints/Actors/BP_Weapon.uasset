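; BP_Weapon is a weapon pickup that bobs vertically until collected and carries its own attack hitbox.
; Construction picks a random skeletal mesh from WeaponsData, and BeginPlay starts a ping-ponging Timeline that sets world Z.
; Sphere overlap stops the bob and restores the origin, then hands a BP_Character the weapon and disables pickup collision.
; OnAttackCheckBegin and OnAttackCheckEnd toggle AttackCollision, initially off, as the attack detection window.
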(event `self.Sphere.OnComponentBeginOverlap`
  (params (OverlappedComponent :type "PrimitiveComponent Object Reference") (OtherActor :type "Actor Object Reference") (OtherComp :type "PrimitiveComponent Object Reference") (OtherBodyIndex :type Integer) (bFromSweep :type Boolean) (SweepResult :type "HitResult Structure (by ref)"))
  (`self.StopWeaponMovement`)
  (`self.K2_SetActorLocation` (`self.orginLocation`) false true)
  (bind _asbp_character (cast `/Game/Blueprints/Character/BP_Character` OtherActor))
  (`/Game/Blueprints/Character/BP_Character.OnWeaponCollected` _asbp_character self)
  (`PrimitiveComponent.SetCollisionEnabled` (`self.Sphere`) "NoCollision"))

(event `OnAttackCheckBegin`
  ; 공격판정 시작
  (`PrimitiveComponent.SetCollisionEnabled` (`self.AttackCollision`) "QueryOnly"))

(event `OnAttackCheckEnd`
  ; 공격판정 종료
  (`PrimitiveComponent.SetCollisionEnabled` (`self.AttackCollision`) "NoCollision"))

(event `self.ReceiveBeginPlay`
  (bind (_returnvalue_x _returnvalue_y) (`KismetMathLibrary.BreakVector` (`self.K2_GetActorLocation`)))
  (set `self.orginLocation` (`self.K2_GetActorLocation`))
  (`PrimitiveComponent.SetCollisionEnabled` (`self.AttackCollision`) "NoCollision")
  (bind (_direction _newtrack_0) (`Timeline|Timeline` :!label _label)
    (:`Update`
      (`self.K2_SetActorLocation` (`KismetMathLibrary.MakeVector` _returnvalue_x _returnvalue_y _newtrack_0)))
    (:`Finished`
      (bind _output_get (set `self.IsUp` (not (`self.IsUp`))))
      (if _output_get
        (goto _label :!via `Reverse`)
        (else
          (goto _label :!via `PlayFromStart`))))))

(event `StopWeaponMovement`
  (goto _label :!via `Stop`))

(fn `UserConstructionScript`
  (bind _weaponappearance (break `/Game/Blueprints/Actors/WeaponsData` (`self.WeaponsData`)))
  (`SkeletalMeshComponent.SetSkeletalMeshAsset` (`self.Mesh`) (`|GetArrayItem` _weaponappearance (`KismetMathLibrary.RandomIntegerInRange` 0 (- (`KismetArrayLibrary.Array_Length` _weaponappearance) 1)))))